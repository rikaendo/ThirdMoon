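; Player pawn that turns by mouse drag and travels over the surface of BP_Moon.
; Releasing a left-mouse drag plays timelines that ease the capsule's yaw toward an angle derived from the drag.
; Holding right mouse rotates the MoonCenterRef pivot by the arrow's forward vector, then line-traces toward the moon's center to place the capsule on the hit point.
; Debug lines and prints remain, and surface-normal alignment logic is present but never runs.
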(event `self.ReceiveBeginPlay`
  (bind _outactors (`GameplayStatics.GetAllActorsOfClass` "/Game/Blueprints/BP_Moon.BP_Moon_C"))
  (set `self.BP_Moon_Ref` (`|GetArrayItem` _outactors))
  (bind _outactors_2 (`GameplayStatics.GetAllActorsOfClass` "/Game/Blueprints/BP_TestOBJ.BP_TestOBJ_C"))
  (set `self.LineTraceIgnoreActors` _outactors_2)
  (set `self.MoonCenterRefRotation` (`SceneComponent.K2_GetComponentRotation` (`self.MoonCenterRef`))))

(event `self.ReceiveTick`
  (params (DeltaSeconds :type "Float (single-precision)"))
  (bind (_returnvalue_roll _returnvalue_pitch) (`KismetMathLibrary.BreakRotator` (`self.K2_GetActorRotation`)))
  (bind (_returnvalue_roll_2 _returnvalue_pitch_2) (`KismetMathLibrary.BreakRotator` (`self.K2_GetActorRotation`)))
  (bind (_returnvalue_roll_3 _returnvalue_pitch_3 _returnvalue_yaw) (`KismetMathLibrary.BreakRotator` (`self.K2_GetActorRotation`)))
  (bind (_returnvalue_roll_4 _returnvalue_pitch_4 _returnvalue_yaw_2) (`KismetMathLibrary.BreakRotator` (`self.K2_GetActorRotation`)))
  (bind (_currentdirection_roll _currentdirection_pitch _currentdirection_yaw) (`KismetMathLibrary.BreakRotator` (`self.CurrentDirection`)))
  (bind _capsule (`self.Capsule`))
  (bind (_currentdirection_roll_2 _currentdirection_pitch_2 _currentdirection_yaw_2) (`KismetMathLibrary.BreakRotator` (`self.CurrentDirection`)))
  (bind (_currentdirection_roll_3 _currentdirection_pitch_3 _currentdirection_yaw_3) (`KismetMathLibrary.BreakRotator` (`self.CurrentDirection`)))
  (bind _mouseinputstart (`self.MouseInputStart`))
  (bind _mouseinputend (`self.MouseInputEnd`))
  (bind (_mooncenterrefrotation_roll _mooncenterrefrotation_pitch) (`KismetMathLibrary.BreakRotator` (`self.MoonCenterRefRotation`)))
  (bind _arrow (`self.Arrow`))
  (bind _returnvalue (- _mouseinputstart _mouseinputend))
  (bind _returnvalue_2 (`SceneComponent.K2_GetComponentLocation` _arrow))
  (bind (_returnvalue_roll_5 _returnvalue_pitch_5 _returnvalue_yaw_3) (`KismetMathLibrary.BreakRotator` (`KismetMathLibrary.MakeRotFromXY` _returnvalue _returnvalue)))
  (bind (_returnvalue_x _returnvalue_y) (`KismetMathLibrary.BreakVector` (* (`KismetMathLibrary.GetForwardVector` (`SceneComponent.RelativeRotation` (`self.Arrow`))) 0.5)))
  (bind _returnvalue_3 (- _mooncenterrefrotation_pitch _returnvalue_x))
  (bind _returnvalue_4 (+ _mooncenterrefrotation_roll _returnvalue_y))
  (bind (_returnvalue_roll_6 _returnvalue_pitch_6) (`KismetMathLibrary.BreakRotator` (`KismetMathLibrary.RInterpTo` (`KismetMathLibrary.MakeRotator` _mooncenterrefrotation_roll _mooncenterrefrotation_pitch _currentdirection_yaw_3) (`KismetMathLibrary.MakeRotator` _returnvalue_4 _returnvalue_3 _currentdirection_yaw_3) (`GameplayStatics.GetWorldDeltaSeconds`) 5.0)))
  (`|ExecutionSequence`
    (:`then_0`
      ;[1 1 1] Turns pawn in direction of mouse drag&release
      (if (`self.bLeftMouseButtonDown`)
        _
        (elif (!= _mouseinputstart _mouseinputend :`ErrorTolerance` 0.001)
          (if (< _returnvalue_yaw_3 -90.0)
            (bind (_direction _deltatime) (`Timeline|Timeline_0` :!via `PlayFromStart`)
              (:`Update`
                (bind _returnvalue_5 (`KismetMathLibrary.FInterpTo` _currentdirection_yaw (+ (+ _returnvalue_yaw_3 270.0) _returnvalue_yaw) _deltatime 5.0))
                (`SceneComponent.K2_SetRelativeRotation` _capsule (`KismetMathLibrary.MakeRotator` 0.0 0.0 _returnvalue_5) false false)
                (set `self.CurrentDirection` (`KismetMathLibrary.MakeRotator` _returnvalue_roll_2 _returnvalue_pitch_2 _returnvalue_5))))
            (else
              (bind (_direction_2 _deltatime_2) (`Timeline|FinterpTimeline` :!via `PlayFromStart`)
                (:`Update`
                  (bind _returnvalue_6 (`KismetMathLibrary.FInterpTo` _currentdirection_yaw_2 (+ (- _returnvalue_yaw_3 90.0) _returnvalue_yaw_2) _deltatime_2 5.0))
                  (`SceneComponent.K2_SetRelativeRotation` _capsule (`KismetMathLibrary.MakeRotator` 0.0 0.0 _returnvalue_6) false false)
                  (set `self.CurrentDirection` (`KismetMathLibrary.MakeRotator` _returnvalue_roll _returnvalue_pitch _returnvalue_6)))))))))
    (:`then_1`
      (if (`self.bRightMouseButtonDown`)
        ;[1 1 1] draw debug line
        (`KismetSystemLibrary.DrawDebugLine` _returnvalue_2 (+ _returnvalue_2 (* (`KismetMathLibrary.GetForwardVector` (`SceneComponent.RelativeRotation` _arrow)) 100.0)) (struct :`R` 0.061365 :`G` 1.0 :`A` 1.0) 100.0 10.0)
        (`SceneComponent.K2_SetWorldRotation` (`self.MoonCenterRef`) (`KismetMathLibrary.MakeRotator` _returnvalue_roll_6 _returnvalue_pitch_6 _currentdirection_yaw_3) false false)
        (bind _output_get (set `self.MoonCenterRefRotation` (`KismetMathLibrary.MakeRotator` _returnvalue_4 _returnvalue_3 _currentdirection_yaw_3)))
        (`KismetSystemLibrary.PrintString` (`KismetStringLibrary.Conv_RotatorToString` _output_get))
        (bind _outhit (`KismetSystemLibrary.LineTraceSingleForObjects` (`SceneComponent.K2_GetComponentLocation` (`self.Arrow`)) (`self.K2_GetActorLocation` (`self.BP_Moon_Ref`)) (`self.LineTraceObjects`) false (`self.LineTraceIgnoreActors`) "ForDuration"))
        (`SceneComponent.K2_SetWorldLocation` (`self.Capsule`) (`.ImpactPoint` (`GameplayStatics.BreakHitResult` _outhit)) false false)))))

(event `Key|LeftMouseButton`
  (params (Key :type "Key Structure"))
  (bind (_locationx _locationy) (`PlayerController.GetMousePosition` (`GameplayStatics.GetPlayerController` 0)))
  (bind (_locationx_2 _locationy_2) (`PlayerController.GetMousePosition` (`GameplayStatics.GetPlayerController` 0)))
  (:`Pressed`
    ;[1 1 1] Reset Mouse Input variables
    (set `self.MouseInputStart` (0.0 0.0 0.0))
    (set `self.MouseInputEnd` (0.0 0.0 0.0))
    (set `self.bLeftMouseButtonDown` true)
    (set `self.MouseInputStart` (`KismetMathLibrary.MakeVector` _locationx _locationy)))
  (:`Released`
    (set `self.bLeftMouseButtonDown` false)
    (set `self.MouseInputEnd` (`KismetMathLibrary.MakeVector` _locationx_2 _locationy_2))))

(event `Key|RightMouseButton`
  (params (Key :type "Key Structure"))
  (:`Pressed`
    (set `self.bRightMouseButtonDown` true)
    (`KismetSystemLibrary.PrintString` "RMB clicked"))
  (:`Released`
    (set `self.bRightMouseButtonDown` false)))

(fn `UserConstructionScript`)