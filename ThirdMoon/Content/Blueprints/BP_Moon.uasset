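; Moon actor that acts as a point gravity source and takes over the first player's view and input on BeginPlay.
; Every Tick it pushes all BP_TestOBJ boxes toward GravityPoint by adding velocity, while overwriting BP_PlayerPawn box velocity with a stronger pull, neither scaled by delta time.
; Turn and LookUp axes rotate the gimbal and camera for debugging.
; GetSurfaceNormal returns the outward direction from the moon's origin to a given location.
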(event `self.ReceiveBeginPlay`
  (bind _returnvalue (`GameplayStatics.GetPlayerController` 0))
  (`PlayerController.SetViewTargetWithBlend` _returnvalue self 0.0 "VTBlend_Linear" 0.0 false)
  (`self.EnableInput` _returnvalue))

(event `self.ReceiveTick`
  (params (DeltaSeconds :type "Float (single-precision)"))
  ;[1 1 1] Point gravity
  (`|ExecutionSequence`
    (:`then_0`
      (bind _outactors (`GameplayStatics.GetAllActorsOfClass` "/Game/Blueprints/BP_TestOBJ.BP_TestOBJ_C")))
    (:`then_1`
      (bind _outactors_2 (`GameplayStatics.GetAllActorsOfClass` "/Game/Blueprints/BP_PlayerPawn.BP_PlayerPawn_C")))
    (:`then_2`
      (`|ExecutionSequence`
        (:`then_0`
          (for _array_element _outactors
            (bind _box (`/Game/Blueprints/BP_TestOBJ.Box` _array_element))
            (`PrimitiveComponent.SetPhysicsLinearVelocity` _box (* (`KismetMathLibrary.GetForwardVector` (`KismetMathLibrary.FindLookAtRotation` (`SceneComponent.K2_GetComponentLocation` _box) (`SceneComponent.K2_GetComponentLocation` (`self.GravityPoint`)))) 9.8) true "None")))
        (:`then_1`
          (for _array_element_2 _outactors_2
            (bind _returnvalue (`self.GetComponentByClass` _array_element_2 "/Script/Engine.BoxComponent"))
            (`PrimitiveComponent.SetPhysicsLinearVelocity` _returnvalue (* (`KismetMathLibrary.GetForwardVector` (`KismetMathLibrary.FindLookAtRotation` (`SceneComponent.K2_GetComponentLocation` _returnvalue) (`SceneComponent.K2_GetComponentLocation` (`self.GravityPoint`)))) 98.0) false "None")))))))

(event `InputAxis|Turn`
  (params (AxisValue :type "Float (single-precision)"))
  ;[1 1 1] Keyboard Camera Input (FOR DEBUGGING PURPOSES ONLY)
  (`SceneComponent.K2_AddLocalRotation` (`self.CameraGimbal`) (`KismetMathLibrary.MakeRotator` 0.0 0.0 (* AxisValue (`GameplayStatics.GetWorldDeltaSeconds`) 30.0)) false false))

(event `InputAxis|LookUp`
  (params (AxisValue :type "Float (single-precision)"))
  ;[1 1 1] Keyboard Camera Input (FOR DEBUGGING PURPOSES ONLY)
  (`SceneComponent.K2_AddLocalRotation` (`self.MoonCamera`) (`KismetMathLibrary.MakeRotator` 0.0 (* AxisValue (`GameplayStatics.GetWorldDeltaSeconds`) 30.0)) false false))

(fn `GetSurfaceNormal`
  (params (PlayerLocation :type "Vector Structure"))
  (returns (SurfaceNormal :type "Vector Structure"))
  (return (`KismetMathLibrary.Normal` (- PlayerLocation (`self.K2_GetActorLocation`)))))

(fn `UserConstructionScript`)