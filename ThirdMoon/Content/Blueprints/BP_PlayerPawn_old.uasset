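; Player pawn that the mouse moves and turns on the surface of a BP_Moon actor through drag-and-release input.
; On left mouse release it applies a local Y offset, then sets roll and pitch from the moon's surface normal and yaw from the drag direction.
; The interp nodes run once per release rather than on Tick.
; An unconnected older block handles drag-based turning and stores CurrentDirection.
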(event `self.ReceiveBeginPlay`
  (bind _outactors (`GameplayStatics.GetAllActorsOfClass` "/Game/Blueprints/BP_Moon.BP_Moon_C"))
  (set `self.BP_Moon_Ref` (`|GetArrayItem` _outactors)))

(event `self.ReceiveTick`
  (params (DeltaSeconds :type "Float (single-precision)")))

(event `Key|LeftMouseButton`
  (params (Key :type "Key Structure"))
  (bind (_returnvalue_roll _returnvalue_pitch _returnvalue_yaw) (`KismetMathLibrary.BreakRotator` (`self.K2_GetActorRotation`)))
  (bind (_returnvalue_roll_2 _returnvalue_pitch_2 _returnvalue_yaw_2) (`KismetMathLibrary.BreakRotator` (`self.K2_GetActorRotation`)))
  (bind _returnvalue (`self.K2_GetActorLocation`))
  (bind (_locationx _locationy) (`PlayerController.GetMousePosition` (`GameplayStatics.GetPlayerController` 0)))
  (bind _returnvalue_2 (- (`self.MouseInputStart`) (`self.MouseInputEnd`)))
  (bind _returnvalue_3 (`KismetMathLibrary.VInterpTo` _returnvalue (0.0 0.0 0.0) (`GameplayStatics.GetWorldDeltaSeconds`) 0.0))
  (bind (_locationx_2 _locationy_2) (`PlayerController.GetMousePosition` (`GameplayStatics.GetPlayerController` 0)))
  (bind (_returnvalue_roll_3 _returnvalue_pitch_3 _returnvalue_yaw_3) (`KismetMathLibrary.BreakRotator` (`KismetMathLibrary.MakeRotFromXY` _returnvalue_2 _returnvalue_2)))
  (:`Pressed`
    (set `self.MouseInputStart` (`KismetMathLibrary.MakeVector` _locationx _locationy)))
  (:`Released`
    (set `self.MouseInputEnd` (`KismetMathLibrary.MakeVector` _locationx_2 _locationy_2))
    (`self.K2_AddActorLocalOffset` (`KismetMathLibrary.MakeVector` 0.0 (`KismetMathLibrary.FInterpTo` 0.0 (`self.MoveDistance`) (`GameplayStatics.GetWorldDeltaSeconds`) 7.0)))
    ;[1 1 1] pawn moves while standing in direction of face normals
    (bind _surfacenormal (`/Game/Blueprints/BP_Moon.GetSurfaceNormal` (`self.BP_Moon_Ref`) _returnvalue))
    (if (< _returnvalue_yaw_3 -90.0)
      (bind (_returnvalue_roll_4 _returnvalue_pitch_4) (`KismetMathLibrary.BreakRotator` (`KismetMathLibrary.MakeRotFromZX` _surfacenormal (`self.GetActorForwardVector`))))
      (`self.K2_SetActorLocationAndRotation` _returnvalue_3 (`KismetMathLibrary.MakeRotator` _returnvalue_roll_4 _returnvalue_pitch_4 (`KismetMathLibrary.FInterpTo` _returnvalue_yaw_2 (+ _returnvalue_yaw_3 270.0) 0.0 7.0)))
      (else
        (`self.K2_SetActorLocationAndRotation` _returnvalue_3 (`KismetMathLibrary.MakeRotator` _returnvalue_roll_4 _returnvalue_pitch_4 (`KismetMathLibrary.FInterpTo` _returnvalue_yaw (- _returnvalue_yaw_3 90.0) 0.0 7.0)))))))

(fn `UserConstructionScript`)